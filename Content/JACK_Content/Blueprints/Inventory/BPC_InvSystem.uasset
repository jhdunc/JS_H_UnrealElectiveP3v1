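; Player inventory component, based on a tutorial, that handles item interaction, stacking, slot transfers and dropping.
; Each tick a forward sphere trace sets the look-at actor, and Interact messages its BPC_ItemData through a server event.
; Items fill a fixed-size slot array, with stack limits and drop classes read from the ItemData table.
; Removals and slot swaps fire an update dispatcher through MC_Update, and dropped items spawn at randomized ground-traced points ahead.
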(event Custom|Server_Interact
  (params (Target :type Actor%20Object%20Reference))
  (bind _returnvalue (Actor|GetComponentbyClass Target "/Game/JACK_Content/Blueprints/Inventory/BPC_ItemData.BPC_ItemData_C"))
  ;[0 0 0 0.005] Inventory System Tutorial:
  ; Credit: https://www.youtube.com/watch?v=4bXYl11sFew&list
  ;;[0 0 0 0] In Case of Multiplayer
  ;;[0 0 0 0] Check if Item (i.e. can pick up)
  (Utilities|IsValid _returnvalue
    (:Is%20Valid
      (Class|BPIInteractable|Interactwith(Message) _returnvalue (Variables|Default|GetPlayerRef)))))

(event Custom|MC_Update
  (Default|CallOnInventoryUpdated))

(event Custom|SERVER_TransferSlots
  (params (SourceInventory :type BPC%20Inv%20System%20Object%20Reference) (SourceIndex :type Integer) (DestinationIndex :type Integer))
  (CallFunction|TransferSlots SourceInventory SourceIndex DestinationIndex))

(event Custom|SERVER_Remove
  (params (Index :type Integer) (RemoveAll :type Boolean) (IsConsumed :type Boolean))
  (CallFunction|RemovefromInventory Index RemoveAll IsConsumed))

(event Custom|SERVER_DropItem
  (params (ItemID :type Name) (Qty :type Integer))
  (for _index (range 0 (- Qty 1))
    (Game|SpawnActorfromClass (.ItemClass (Utilities|Struct|BreakFItemStruct (CallFunction|GetItemData ItemID))) (Math|Transform|MakeTransform (CallFunction|GetDropLocation) "0, 0, 0" "1.000000,1.000000,1.000000") "Undefined" "MultiplyWithRoot" 0 0)))

(event Input|EnhancedActionEvents|EnhancedInputActionIA_Interact
  (params (ActionValue :type Boolean) (ElapsedSeconds :type Float%20%28double-precision%29) (TriggeredSeconds :type Float%20%28double-precision%29) (InputAction :type Input%20Action%20Object%20Reference :default "/Game/JACK_Content/Input/Actions/IA_Interact.IA_Interact"))
  ;[0 0 0 0.005] Inventory System Tutorial:
  ; Credit: https://www.youtube.com/watch?v=4bXYl11sFew&list
  (bind _lookatactor (Variables|Default|GetLookAtActor)
    (:then
      (CallFunction|ServerInteract _lookatactor))
    (:else)))

(event EventTick
  (params (DeltaSeconds :type Float%20%28single-precision%29))
  ;[0 0 0 0.005] Inventory System Tutorial:
  ; Credit: https://www.youtube.com/watch?v=4bXYl11sFew&list
  (CallFunction|InteractionTrace))

(event EventBeginPlay
  ;[0 0 0 0.005] Inventory System Tutorial:
  ; Credit: https://www.youtube.com/watch?v=4bXYl11sFew&list
  ;;[0.9569 0.1216 0 0.2235] Get Player Reference (to use instead of Camera)
  (bind _asbp_third_person_character (Utilities|Casting|CastToBP_ThirdPersonCharacter (Game|GetPlayerCharacter 0)))
  (Variables|Default|SetPlayerRef _asbp_third_person_character)
  (Utilities|Array|Resize (Variables|Default|GetContent) (Variables|Default|GetInventorySize)))

(event Input|KeyboardEvents|1
  (params (Key :type Key%20Structure :default "None"))
  (:Pressed
    (CallFunction|DEBUGPrintContents)))

(fn AddtoInventory
  (params (ItemID :type Name) (Qty :type Integer))
  ;[0 0 0 0] For every item, find appropriate slot in inventory
  (LocalVariables|SetLocal_QtyRemain Qty)
  (while (and (> (LocalVariables|GetLocal_QtyRemain) 0) (not (LocalVariables|GetLocal_HasFailed)))
    (bind (_index _foundslot) (CallFunction|FindSlot ItemID))
    ;[0 0 0 0] If Inventory Slot Exists with Item, Add to Stack
    (if _foundslot
      (CallFunction|AddtoStack _index 1)
      (Math|Integer|DecrementInt (LocalVariables|GetLocal_QtyRemain))
      (else
        ;[0 0 0 0] If No Existing Item, Create new stack
        (if (.HasEmptySlot (CallFunction|CheckforEmptySlots))
          (bind _success (CallFunction|CreateNewStack ItemID 1))
          (if _success
            (Math|Integer|DecrementInt (LocalVariables|GetLocal_QtyRemain))
            (else
              (LocalVariables|SetLocal_HasFailed true)))
          (else
            (LocalVariables|SetLocal_HasFailed false))))))
  (return (not (LocalVariables|GetLocal_HasFailed)) (LocalVariables|GetLocal_QtyRemain)))

(fn RemovefromInventory
  (params (Index :type Integer) (RemoveAll :type Boolean) (IsConsumed :type Boolean))
  (bind _content (Variables|Default|GetContent))
  (bind _content_2 (Variables|Default|GetContent))
  (bind _output (Utilities|Array|Get(acopy) _content Index))
  (bind _output_2 (Utilities|Array|Get(acopy) _content_2 Index))
  (LocalVariables|SetLocalItem (.itemid _output))
  (LocalVariables|SetLocalQty (.qty _output))
  (Utilities|FlowControl|Sequence
    (:then_0
      (if (or RemoveAll (== (LocalVariables|GetLocalQty) 1))
        (Utilities|Array|SetArrayElem (Variables|Default|GetContent) Index (Utilities|Struct|MakeFSlotStruct "" 0))
        (if (not IsConsumed)
          (CallFunction|SERVERDropItem (LocalVariables|GetLocalItem) (LocalVariables|GetLocalQty)))
        (else
          ;[0 0 0 0] Drop 1 with Stack Remaining
          (Utilities|Struct|SetmembersinFSlotStruct _output_2 (- (.Qty (Utilities|Struct|BreakFSlotStruct _output_2)) 1))
          (if (not IsConsumed)
            (CallFunction|SERVERDropItem (LocalVariables|GetLocalItem) 1)))))
    (:then_1
      (CallFunction|MCUpdate))))

(fn InteractionTrace
  (bind _playerref (Variables|Default|GetPlayerRef))
  (bind _returnvalue (Transformation|GetActorLocation _playerref))
  ;[0 0 0 0] Create Sphere Trace to Look For Interactable Objects
  (bind (_outhit _returnvalue_2) (Collision|SphereTraceByChannel _returnvalue (+ _returnvalue (* (Transformation|GetActorForwardVector _playerref) (Variables|Default|GetRange))) 4e+01 "TraceTypeQuery1" false (Utilities|Array|MakeArray (Components|GetOwner)) "None"))
  (if _returnvalue_2
    (if (!= (Variables|Default|GetLookAtActor) (.HitActor (Collision|BreakHitResult _outhit)))
      (bind _output_get (Variables|Default|SetLookAtActor (.HitActor (Collision|BreakHitResult _outhit))))
      (bind _message (Class|BPIInteractable|Lookat(Message) _output_get))
      (Development|PrintString _message))
    (else
      (Variables|Default|SetLookAtActor 0))))

(fn FindSlot
  (params (ItemID :type Name))
  ;[0 0 0 0] Look for Existing Item, Verify not at Max Qty
  (for (_array_element _array_index) (Variables|Default|GetContent)
    (if (== (.ItemID (Utilities|Struct|BreakFSlotStruct _array_element)) ItemID)
      (if (< (.Qty (Utilities|Struct|BreakFSlotStruct _array_element)) (CallFunction|GetMaxStackSize ItemID))
        (return _array_index true))))
  (return -1 false))

(fn GetMaxStackSize
  (params (ItemID :type Name))
  ;[0 0 0 0] pull info from data table
  (bind _returnvalue (Utilities|GetDataTableRow "/Game/JACK_Content/Blueprints/Inventory/NotJacksWork/ItemData.ItemData" ItemID)
    (:then
      (return (Utilities|Struct|BreakFItemStruct _returnvalue)))
    (:RowNotFound
      (return -1))))

(fn AddtoStack
  (params (Index :type Integer) (Qty :type Integer))
  (bind _content (Variables|Default|GetContent))
  (bind _output (Utilities|Array|Get(acopy) _content Index))
  ;[0 0 0 0] From Tutorial
  (Utilities|Array|SetArrayElem (Variables|Default|GetContent) Index (Utilities|Struct|MakeFSlotStruct (.itemid _output) (+ (.qty _output) Qty))))

(fn CheckforEmptySlots
  ;[0 0 0 0] from Tutorial
  (for (_array_element _array_index) (Variables|Default|GetContent)
    (if (== (.Qty (Utilities|Struct|BreakFSlotStruct _array_element)) 0)
      (return true _array_index)))
  (return false -1))

(fn CreateNewStack
  (params (ItemID :type Name) (Qty :type Integer))
  (bind (_hasemptyslot _emptyindex) (CallFunction|CheckforEmptySlots))
  ;[0 0 0 0] from Tutorial
  (if _hasemptyslot
    (Utilities|Array|SetArrayElem (Variables|Default|GetContent) _emptyindex (Utilities|Struct|MakeFSlotStruct ItemID Qty))
    (return true)
    (else
      (return false))))

(fn DEBUGPrintContents
  (for (_array_element _array_index) (Variables|Default|GetContent)
    (Development|PrintString (Utilities|String|Append (Utilities|String|ToString(Integer) _array_index) ": " (Utilities|String|ToString(Name) (.ItemID (Utilities|Struct|BreakFSlotStruct _array_element))) " = " (Utilities|String|ToString(Integer) (.Qty (Utilities|Struct|BreakFSlotStruct _array_element)))))))

(fn TransferSlots
  (params (SourceInventory :type BPC%20Inv%20System%20Object%20Reference) (SourceIndex :type Integer) (DestinationIndex :type Integer))
  ;[0 0 0 0] Drag/Drop Replacement (slot/inventory)
  (LocalVariables|SetLocalSlotContent (Utilities|Array|Get(acopy) (Variables|BPC_InvSystem_C|GetContent SourceInventory) SourceIndex))
  (if (not (< DestinationIndex 0))
    (if (not (== (.ItemID (Utilities|Struct|BreakFSlotStruct (LocalVariables|GetLocalSlotContent))) (.ItemID (Utilities|Struct|BreakFSlotStruct (Utilities|Array|Get(acopy) (Variables|Default|GetContent) DestinationIndex)))))
      (Utilities|Array|SetArrayElem (Variables|BPC_InvSystem_C|GetContent SourceInventory) SourceIndex (Utilities|Array|Get(acopy) (Variables|Default|GetContent) DestinationIndex))
      (Utilities|Array|SetArrayElem (Variables|Default|GetContent) DestinationIndex (LocalVariables|GetLocalSlotContent))
      (CallFunction|MCUpdate)
      (CallFunction|MCUpdate SourceInventory))))

(fn GetItemData
  (params (ItemID :type Name))
  ;[0 0 0 0] from Tutorial
  (bind _returnvalue (Utilities|GetDataTableRow "/Game/JACK_Content/Blueprints/Inventory/NotJacksWork/ItemData.ItemData" ItemID)
    (:then
      (return _returnvalue))))

(fn GetDropLocation
  (bind _returnvalue (Components|GetOwner))
  (bind _returnvalue_2 (Transformation|GetActorLocation _returnvalue))
  (bind _returnvalue_3 (Transformation|GetActorForwardVector _returnvalue))
  (bind _returnvalue_4 (Math|Random|RandomUnitVectorinConeinDegrees _returnvalue_3 3e+01))
  (bind _returnvalue_5 (* _returnvalue_4 1.5e+02))
  (bind _returnvalue_6 (+ _returnvalue_2 _returnvalue_5))
  ;[0 0 0 0] From tutorial: allows randomization of drop all placement
  (bind _outhit (Collision|LineTraceByChannel _returnvalue_6 (- _returnvalue_6 "0.000000,0.000000,500.000000") "TraceTypeQuery1" false 0 "None"))
  (return (.Location (Collision|BreakHitResult _outhit))))