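; BP_LightParent is an inventory light orb item, apparently a base class, that bobs vertically and reports its item name when looked at.
; Two timelines, Bob and BobAgain, alternate forward and reverse to move the Sphere endlessly.
; The construction script creates dynamic materials for the core and wisp, applying color variables to them and to the orbiting insect particles.
; LookAt reads the name from the data table row referenced by BPCItemData.
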(event EventBeginPlay
  ;[0.9569 0.1216 0 0.2235] Set Object Vertical Bob
  (bind _z_axis_move (Timeline|Bob Play)
    (:Update
      (Transformation|SetRelativeLocation (Variables|Default|GetSphere) _z_axis_move false false))
    (:Finished
      (bind _z_axis_move_2 (Timeline|BobAgain ReverseFromEnd)
        (:Update
          (Transformation|SetRelativeLocation (Variables|Default|GetSphere) _z_axis_move_2 false false))
        (:Finished
          (Timeline|Bob PlayFromStart))))))

(event EventTick
  (params (DeltaSeconds :type Float%20%28single-precision%29)))

(fn ConstructionScript
  (bind _trailscolor (Variables|Default|GetTrailsColor))
  (bind _sphere (Variables|Default|GetSphere))
  (bind _wisp (Variables|Default|Getwisp))
  ;[0.9569 0.1216 0 0.2235] Set FX orbit to color
  (Effects|Components|ParticleSystem|SetVectorParameter (Variables|Default|GetPfx_LightInsects1) "LightColor" (Math|Conversions|ToVector(LinearColor) (Variables|Default|GetOrbitColor)))
  ;[0.9569 0.1216 0 0.2235] Create DMIs for Orb materials
  (bind _returnvalue (Rendering|Material|CreateDynamicMaterialInstance _sphere 0 (Rendering|Material|GetMaterial _sphere 0) "None" :!class /Script/Engine.PrimitiveComponent))
  (LocalVariables|SetCoreMat _returnvalue)
  (bind _returnvalue_2 (Rendering|Material|CreateDynamicMaterialInstance _wisp 0 (Rendering|Material|GetMaterial _wisp 0) "None" :!class /Script/Engine.PrimitiveComponent))
  (LocalVariables|SetWispMaterial _returnvalue_2)
  (Rendering|Material|SetVectorParameterValue (LocalVariables|GetCoreMat) "Color" (Variables|Default|GetCoreColor) :!class /Script/Engine.MaterialInstanceDynamic)
  ;[0.9569 0.1216 0 0.2235] Set inner movement color of orb
  (Rendering|Material|SetVectorParameterValue (LocalVariables|GetWispMaterial) "Bot Color" _trailscolor :!class /Script/Engine.MaterialInstanceDynamic)
  (Rendering|Material|SetVectorParameterValue (LocalVariables|GetWispMaterial) "Top Color" _trailscolor :!class /Script/Engine.MaterialInstanceDynamic))

(fn Lookat
  (bind _bpc_itemdata (Variables|Default|GetBPC_ItemData))
  (bind _itemid (Variables|/Game/JACK_Content/Blueprints/Inventory/BPC_ItemData.BPC_ItemData_C|GetItemID _bpc_itemdata))
  ;[0 0 0 0] Return Item Data Name when Object Looked At
  (bind _returnvalue (Utilities|GetDataTableRow (.datatable _itemid) (.rowname _itemid))
    (:then
      (return (.Name (Utilities|Struct|BreakFItemStruct _returnvalue))))))