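; Parent inventory item actor that fades in and flashes an outline when the player is in overlap range and facing it.
; When fading is enabled, Tick checks range and horizontal dot product, with paired DoOnce gates triggering each fade once per change.
; Timelines drive the dynamic material's Color alpha and the overlay outline's thickness through a parameter collection.
; Visible items register with their distance in the player's Viewd map, and leave it when hidden or destroyed.
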(event Custom|FadeIn
  (params (DynamicMaterial :type Material%20Instance%20Dynamic%20Object%20Reference))
  ;[0.9569 0.1216 0 0.2235] Fade Object If in LoS and InRange
  (bind _newtrack_0 (Timeline|TL_Fade PlayFromStart)
    (:Update
      (bind _returnvalue (Rendering|Material|GetVectorParameterValue DynamicMaterial "Color" :!class /Script/Engine.MaterialInstanceDynamic))
      (Rendering|Material|SetVectorParameterValue DynamicMaterial "Color" (Utilities|Struct|MakeLinearColor (.r _returnvalue) (.g _returnvalue) (.b _returnvalue) (Math|Float|Lerp 0.0 1.0 _newtrack_0)) :!class /Script/Engine.MaterialInstanceDynamic))
    (:Finished
      ;[0.9569 0.1216 0 0.2235] Set Outline
      (bind _newtrack_0_2 (Timeline|TL_Outline PlayFromStart)
        (:Update
          (Rendering|Material|SetOverlayMaterial (Variables|Default|GetMesh) (Variables|Default|GetDynamicOverlay) :!class /Script/Engine.MeshComponent)
          (Rendering|Material|SetScalarParameterValue "/Game/JACK_Content/Materials/MPC_OutlineParameters.MPC_OutlineParameters" "LineThickness" (* _newtrack_0_2 3.0) :!class /Script/Engine.KismetMaterialLibrary))
        (:Finished
          (bind _returnvalue_2 (CallFunction|CheckifSeen))
          (if (not _returnvalue_2)
            (Rendering|Material|SetOverlayMaterial (Variables|Default|GetMesh) 0 :!class /Script/Engine.MeshComponent)))))))

(event Custom|FadeOut
  (params (Dynamic%20Material :type Material%20Instance%20Dynamic%20Object%20Reference))
  ;[0.9569 0.1216 0 0.2235] Fade Object If in LoS and InRange
  ;;[1 0.5673 0.4162 0] Turn Off Outline
  (Rendering|Material|SetOverlayMaterial (Variables|Default|GetMesh) 0 :!class /Script/Engine.MeshComponent)
  (bind _newtrack_0 (Timeline|Timeline ReverseFromEnd)
    (:Update
      (bind _returnvalue (Rendering|Material|GetVectorParameterValue Dynamic%20Material "Color" :!class /Script/Engine.MaterialInstanceDynamic))
      (Rendering|Material|SetVectorParameterValue Dynamic%20Material "Color" (Utilities|Struct|MakeLinearColor (.r _returnvalue) (.g _returnvalue) (.b _returnvalue) (Math|Float|Lerp 0.0 1.0 _newtrack_0)) :!class /Script/Engine.MaterialInstanceDynamic))))

(event Custom|Fade%20Check
  (bind _materialinst (Variables|Default|GetMaterialInst))
  ;[0.9569 0.1216 0 0.2235] Fade Logic
  ;;[0 0 0 0] Determine if object within view angle
  (bind _returnvalue (CallFunction|CheckifSeen))
  (if _returnvalue
    (Utilities|FlowControl|DoOnce false :!label _label
      (:Completed
        (CallFunction|Fadein _materialinst)
        ;[0.9569 0.1216 0 0.2235] Add/Remove from Player's "in view" list
        (CallFunction|CheckObj true)
        (goto _label_2 Reset)))
    (else
      (Utilities|FlowControl|DoOnce false :!label _label_2
        (:Completed
          (CallFunction|FadeOut _materialinst)
          (CallFunction|CheckObj false)
          (goto _label Reset))))))

(event EventBeginPlay
  ;[0.9569 0.1216 0 0.2235] Create Dynamic Material Instance
  (bind _returnvalue (Rendering|Material|CreateDynamicMaterialInstance (Variables|Default|GetMesh) 0 0 "None" :!class /Script/Engine.PrimitiveComponent))
  (Variables|Default|SetMaterialInst _returnvalue)
  ;[0.9569 0.1216 0 0.2235] Create Character Reference
  (bind _asbp_third_person_character (Utilities|Casting|CastToBP_ThirdPersonCharacter (Game|GetPlayerCharacter 0)))
  (Variables|Default|SetPlayerRef _asbp_third_person_character)
  (Rendering|Material|SetOverlayMaterial (Variables|Default|GetMesh) 0 :!class /Script/Engine.MeshComponent))

(event Collision|EventActorBeginOverlap
  (params (OtherActor :type Actor%20Object%20Reference))
  ;[0.9569 0.1216 0 0.2235] Set bool if character in collision range
  (if (== OtherActor (Variables|Default|GetPlayerRef))
    (Variables|Default|SetinRange true)))

(event EventTick
  (params (DeltaSeconds :type Float%20%28single-precision%29))
  (if (Variables|Default|GetFadeEnabled)
    (CallFunction|FadeCheck)))

(event EventDestroyed
  (CallFunction|RemovefromNearby))

(event Collision|EventActorEndOverlap
  (params (OtherActor :type Actor%20Object%20Reference))
  ;[0.9569 0.1216 0 0.2235] Set bool if character in collision range
  (if (== OtherActor (Variables|Default|GetPlayerRef))
    (Variables|Default|SetinRange false)))

(fn ConstructionScript
  ;[0.9569 0.1216 0 0.2235] Set dynamic overlay material so parameters can change
  (bind _returnvalue (Rendering|Material|CreateDynamicMaterialInstance "/Game/JACK_Content/Materials/MM_Outline.MM_Outline" "None" "None" :!class /Script/Engine.KismetMaterialLibrary))
  (bind _output_get (Variables|Default|SetDynamicOverlay _returnvalue))
  (Rendering|Material|SetOverlayMaterial (Variables|Default|GetMesh) _output_get :!class /Script/Engine.MeshComponent))

(fn CheckObj
  (params (isVis :type Boolean))
  ;[0.9569 0.1216 0 0.2235] Add/Remove obj to map if in view
  (if isVis
    (CallFunction|AddtoNearby)
    (else
      (CallFunction|RemovefromNearby))))

(fn RemovefromNearby
  ;[0.9569 0.1216 0 0.2235] Remove obj from Nearby
  (Utilities|Map|Remove (Variables|/Game/JACK_Content/Blueprints/BP_ThirdPersonCharacter.BP_ThirdPersonCharacter_C|GetViewd (Variables|Default|GetPlayerRef)) self))

(fn AddtoNearby
  ;[0.9569 0.1216 0 0.2235] Get Obj Distance from Player, add/update Viewd Map
  (Utilities|Map|Add (Variables|/Game/JACK_Content/Blueprints/BP_ThirdPersonCharacter.BP_ThirdPersonCharacter_C|GetViewd (Variables|Default|GetPlayerRef)) self (Math|Float|Truncate (Math|Vector|Distance(Vector) (Transformation|GetActorLocation (Variables|Default|GetPlayerRef)) (Transformation|GetActorLocation)))))

(fn CheckifSeen
  ;[0 0 0 0] Check horizontal dot product to
  (return (and (Math|Float|InRange(Float) (Class|Actor|GetHorizontalDotProductto (Game|GetPlayerCharacter 0) self) 0.0 1.0) (Variables|Default|GetinRange))))

(fn Lookat)