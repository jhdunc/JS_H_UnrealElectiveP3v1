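; Parent Blueprint for a glowing orb item that bobs in place and registers itself as a nearby object for the player.
; Construction tints the orb's dynamic core material, point light and orbiting particles from color variables, while two chained timelines loop the bob.
; Overlap events set an in-range flag, which Tick uses to add the item with its distance to the player's Viewd map or remove it.
; Interact and LookAt are empty stubs.
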(event EventBeginPlay
  (bind _sphere (Variables|Default|GetSphere))
  ;[0.9569 0.1216 0 0.2235] Create Character Reference
  (bind _asbp_third_person_character (Utilities|Casting|CastToBP_ThirdPersonCharacter (Game|GetPlayerCharacter 0)))
  (Variables|Default|SetPlayerRef _asbp_third_person_character)
  (Variables|Default|SetlocalPos (Transformation|GetWorldLocation (Variables|Default|GetSphere)))
  ;[0.9569 0.1216 0 0.2235] Set Object Vertical Bob
  (bind _z_axis_move (Timeline|Timeline Play)
    (:Update
      (Transformation|SetRelativeLocation _sphere (+ (Variables|Default|GetlocalPos) _z_axis_move) false false))
    (:Finished
      (bind _z_axis_move_2 (Timeline|Timeline_0 ReverseFromEnd)
        (:Update
          (Transformation|SetRelativeLocation _sphere (+ (Variables|Default|GetlocalPos) _z_axis_move_2) false false))
        (:Finished
          (Timeline|Timeline PlayFromStart))))))

(event Collision|EventActorBeginOverlap
  (params (OtherActor :type Actor%20Object%20Reference))
  ;[0.9569 0.1216 0 0.2235] Set bool if character in collision range
  (if (== OtherActor (Variables|Default|GetPlayerRef))
    (Variables|Default|SetinRange true)))

(event EventTick
  (params (DeltaSeconds :type Float%20%28single-precision%29))
  (CallFunction|CheckObj (Variables|Default|GetinRange)))

(event EventDestroyed
  (CallFunction|RemovefromNearby))

(event Collision|EventActorEndOverlap
  (params (OtherActor :type Actor%20Object%20Reference))
  ;[0.9569 0.1216 0 0.2235] Set bool if character in collision range
  (if (== OtherActor (Variables|Default|GetPlayerRef))
    (Variables|Default|SetinRange false)))

(event EventInteractwith
  (params (PlayerRef :type BP%20Third%20Person%20Character%20Object%20Reference)))

(fn ConstructionScript
  (bind _sphere (Variables|Default|GetSphere))
  ;[0.9569 0.1216 0 0.2235] Set FX orbit to color
  (Effects|Components|ParticleSystem|SetVectorParameter (Variables|Default|GetPfx_LightInsects1) "LightColor" (Math|Conversions|ToVector(LinearColor) (Variables|Default|GetParticleColor)))
  ;[0.9569 0.1216 0 0.2235] Create DMIs for Orb materials
  (bind _returnvalue (Rendering|Material|CreateDynamicMaterialInstance _sphere 0 (Rendering|Material|GetMaterial _sphere 0) "None" :!class /Script/Engine.PrimitiveComponent))
  (LocalVariables|SetCoreMat _returnvalue)
  (Rendering|Material|SetVectorParameterValue (LocalVariables|GetCoreMat) "Color" (Variables|Default|GetCoreColor) :!class /Script/Engine.MaterialInstanceDynamic)
  (Rendering|Components|Light|SetLightColor (Variables|Default|GetPointLight) (Variables|Default|GetCoreColor) true))

(fn CheckObj
  (params (isVis :type Boolean))
  ;[0.9569 0.1216 0 0.2235] Add/Remove obj to map if in view
  (if isVis
    (CallFunction|AddtoNearby)
    (else
      (CallFunction|RemovefromNearby))))

(fn RemovefromNearby
  ;[0.9569 0.1216 0 0.2235] Remove obj from Nearby
  (Utilities|Map|Remove (Variables|/Game/JACK_Content/Blueprints/BP_ThirdPersonCharacter.BP_ThirdPersonCharacter_C|GetViewd (Variables|Default|GetPlayerRef)) self))

(fn AddtoNearby
  ;[0.9569 0.1216 0 0.2235] Get Obj Distance from Player, add/update Viewd Map
  (Utilities|Map|Add (Variables|/Game/JACK_Content/Blueprints/BP_ThirdPersonCharacter.BP_ThirdPersonCharacter_C|GetViewd (Variables|Default|GetPlayerRef)) self (Math|Float|Truncate (Math|Vector|Distance(Vector) (Transformation|GetActorLocation (Variables|Default|GetPlayerRef)) (Transformation|GetActorLocation)))))

(fn CheckifSeen
  (return (and (Math|Float|InRange(Float) (Class|Actor|GetHorizontalDotProductto (Game|GetPlayerCharacter 0) self) 0.0 1.0) (Variables|Default|GetinRange))))

(fn Lookat)