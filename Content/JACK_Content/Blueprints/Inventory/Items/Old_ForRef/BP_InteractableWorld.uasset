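; Base world interactable actor that registers itself in the player's Viewd map, keyed to its truncated distance, as a nearby object.
; Without fading, overlap begin and end add or remove it.
; With FadeEnabled, Tick checks overlap range and a dot-product view angle, using paired DoOnce gates to trigger timeline-driven alpha fades on a dynamic material and update the map.
; Interaction only prints a debug string, and destruction deregisters the actor.
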(event Custom|FadeIn
  (params (DynamicMaterial :type Material%20Instance%20Dynamic%20Object%20Reference))
  ;[0.9569 0.1216 0 0.2235] Fade Object If in LoS and InRange
  (bind _newtrack_0 (Timeline|fade PlayFromStart)
    (:Update
      (bind _returnvalue (Rendering|Material|GetVectorParameterValue DynamicMaterial "None" :!class /Script/Engine.MaterialInstanceDynamic))
      (Rendering|Material|SetVectorParameterValue DynamicMaterial "Color" (Utilities|Struct|MakeLinearColor (.r _returnvalue) (.g _returnvalue) (.b _returnvalue) (Math|Float|Lerp 0.0 1.0 _newtrack_0)) :!class /Script/Engine.MaterialInstanceDynamic))))

(event Custom|FadeOut
  (params (Dynamic%20Material :type Material%20Instance%20Dynamic%20Object%20Reference))
  ;[0.9569 0.1216 0 0.2235] Fade Object If in LoS and InRange
  (bind _newtrack_0 (Timeline|Timeline ReverseFromEnd)
    (:Update
      (bind _returnvalue (Rendering|Material|GetVectorParameterValue Dynamic%20Material "None" :!class /Script/Engine.MaterialInstanceDynamic))
      (Rendering|Material|SetVectorParameterValue Dynamic%20Material "Color" (Utilities|Struct|MakeLinearColor (.r _returnvalue) (.g _returnvalue) (.b _returnvalue) (Math|Float|Lerp 0.0 1.0 _newtrack_0)) :!class /Script/Engine.MaterialInstanceDynamic))))

(event Custom|Fade%20Check
  (bind _spheremat (Variables|Default|GetSphereMat))
  ;[0.9569 0.1216 0 0.2235] Fade Logic
  (if (and (Math|Float|InRange(Float) (Class|Actor|GetHorizontalDotProductto (Game|GetPlayerCharacter 0) self) 0.0 1.0) (Variables|Default|GetinRange))
    (Utilities|FlowControl|DoOnce false :!label _label
      (:Completed
        (CallFunction|Fadein _spheremat)
        ;[0.9569 0.1216 0 0.2235] Add/Remove from Player's "in view" list
        (CallFunction|CheckObj true)
        (goto _label_2 Reset)))
    (else
      (Utilities|FlowControl|DoOnce false :!label _label_2
        (:Completed
          (CallFunction|FadeOut _spheremat)
          (CallFunction|CheckObj false)
          (goto _label Reset))))))

(event EventBeginPlay
  ;[0.9569 0.1216 0 0.2235] Create Dynamic Material Instance
  (bind _returnvalue (Rendering|Material|CreateDynamicMaterialInstance (Variables|Default|GetMesh) 0 0 "None" :!class /Script/Engine.PrimitiveComponent))
  (Variables|Default|SetSphereMat _returnvalue)
  ;[0.9569 0.1216 0 0.2235] Create Character Reference
  (bind _asbp_third_person_character (Utilities|Casting|CastToBP_ThirdPersonCharacter (Game|GetPlayerCharacter 0)))
  (Variables|Default|SetPlayerRef _asbp_third_person_character))

(event Collision|EventActorBeginOverlap
  (params (OtherActor :type Actor%20Object%20Reference))
  ;[0.9569 0.1216 0 0.2235] Set bool if character in collision range
  (if (== OtherActor (Variables|Default|GetPlayerRef))
    (Variables|Default|SetinRange true)
    ;[1 1 1] If obj does not fade, add/remove
    (if (not (Variables|Default|GetFadeEnabled))
      (CallFunction|AddtoNearby))))

(event EventTick
  (params (DeltaSeconds :type Float%20%28single-precision%29))
  ;[0.9569 0.1216 0 0.2235] If Object fades, run fade logic
  (if (Variables|Default|GetFadeEnabled)
    (CallFunction|FadeCheck)))

(event EventDestroyed
  (CallFunction|RemovefromNearby))

(event Collision|EventActorEndOverlap
  (params (OtherActor :type Actor%20Object%20Reference))
  ;[0.9569 0.1216 0 0.2235] Set bool if character in collision range
  (if (== OtherActor (Variables|Default|GetPlayerRef))
    (Variables|Default|SetinRange false)
    ;[1 1 1] If obj does not fade, add/remove
    (if (not (Variables|Default|GetFadeEnabled))
      (CallFunction|RemovefromNearby))))

(event EventInteractwith
  (params (PlayerRef :type BP%20Third%20Person%20Character%20Object%20Reference))
  (Development|PrintString "I have interacted"))

(fn ConstructionScript)

(fn CheckObj
  (params (isVis :type Boolean))
  ;[0.9569 0.1216 0 0.2235] Add/Remove obj to map if in view
  (if isVis
    (CallFunction|AddtoNearby)
    (else
      (CallFunction|RemovefromNearby))))

(fn RemovefromNearby
  ;[0.9569 0.1216 0 0.2235] Remove obj from Nearby
  (Utilities|Map|Remove (Variables|/Game/JACK_Content/Blueprints/BP_ThirdPersonCharacter.BP_ThirdPersonCharacter_C|GetViewd (Variables|Default|GetPlayerRef)) self))

(fn AddtoNearby
  ;[0.9569 0.1216 0 0.2235] Get Obj Distance from Player, add/update Viewd Map
  (Utilities|Map|Add (Variables|/Game/JACK_Content/Blueprints/BP_ThirdPersonCharacter.BP_ThirdPersonCharacter_C|GetViewd (Variables|Default|GetPlayerRef)) self (Math|Float|Truncate (Math|Vector|Distance(Vector) (Transformation|GetActorLocation (Variables|Default|GetPlayerRef)) (Transformation|GetActorLocation)))))

(fn Lookat)