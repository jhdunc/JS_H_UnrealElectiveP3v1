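; Helper for inventory items that tracks whether an item is near and in front of the player.
; VisSetup supplies the item, player and mesh references, and overlap events toggle an in-range flag for the player.
; CheckIfSeen combines that flag with a horizontal dot product test.
; CheckObj adds or removes the item in the player's Viewd map, keyed by actor with truncated distance as value.
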(event Custom|VisSetup
  (params (ActorRef :type Actor%20Object%20Reference) (PlayerRef :type BP%20Third%20Person%20Character%20Object%20Reference) (MeshRef :type Static%20Mesh%20Component%20Object%20Reference))
  (Variables|Default|SetActorRef ActorRef)
  (Variables|Default|SetPlayerRef PlayerRef)
  (Variables|Default|SetStaticMesh MeshRef))

(event Custom|OverlapEnter
  (params (OtherActor :type Actor%20Object%20Reference))
  ;[0.9569 0.1216 0 0.2235] Set bool if character in collision range
  (if (== OtherActor (Variables|Default|GetPlayerRef))
    (Variables|Default|SetinRange true)))

(event Custom|OverlapExit
  (params (OtherActor :type Actor%20Object%20Reference))
  ;[0.9569 0.1216 0 0.2235] Set bool if character in collision range
  (if (== OtherActor (Variables|Default|GetPlayerRef))
    (Variables|Default|SetinRange false)))

(event EventBeginPlay
  ;[0.9569 0.1216 0 0.2235] Create Dynamic Material Instance
  (Utilities|FlowControl|Delay 0.2)
  (bind _returnvalue (Rendering|Material|CreateDynamicMaterialInstance (Variables|Default|GetStaticMesh) 0 0 "None" :!class /Script/Engine.PrimitiveComponent))
  (Variables|Default|SetSM_Inst _returnvalue)
  (Rendering|Material|SetOverlayMaterial (Variables|Default|GetStaticMesh) 0 :!class /Script/Engine.MeshComponent))

(event EventTick
  (params (DeltaSeconds :type Float%20%28single-precision%29)))

(fn AddNearby
  (params (ObjSeen :type Actor%20Object%20Reference))
  (bind _playerref (Variables|Default|GetPlayerRef))
  ;[0.9569 0.1216 0 0.2235] Get Obj Distance from Player, add/update Viewd Map
  (Utilities|Map|Add (Variables|/Game/JACK_Content/Blueprints/BP_ThirdPersonCharacter.BP_ThirdPersonCharacter_C|GetViewd _playerref) ObjSeen (Math|Float|Truncate (Math|Vector|Distance(Vector) (Transformation|GetActorLocation _playerref) (Transformation|GetActorLocation ObjSeen)))))

(fn RemoveNearby
  ;[0.9569 0.1216 0 0.2235] Remove obj from Nearby
  (Utilities|Map|Remove (Variables|/Game/JACK_Content/Blueprints/BP_ThirdPersonCharacter.BP_ThirdPersonCharacter_C|GetViewd (Variables|Default|GetPlayerRef)) (Variables|Default|GetActorRef)))

(fn CheckObj
  (params (isVis :type Boolean))
  ;[0.9569 0.1216 0 0.2235] Add/Remove Obj from Map if Seen/NotSeen
  (if isVis
    (CallFunction|AddNearby (Variables|Default|GetActorRef))
    (else
      (CallFunction|RemoveNearby))))

(fn CheckifSeen
  ;[0 0 0 0] Check horizontal dot product to
  (return (and (Math|Float|InRange(Float) (Class|Actor|GetHorizontalDotProductto (Game|GetPlayerCharacter 0) (Variables|Default|GetActorRef)) 0.0 1.0) (Variables|Default|GetinRange))))