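; BPC_ItemData is an item component that makes its owning actor a collectable the player can pick up into their inventory.
; At BeginPlay it enables replication on the owner, then waits a tick to cache the first WB_InventoryGrid widget found.
; Interaction adds the item ID and quantity to the player's BPCInvSystem and, on success, refreshes the grid, zeroes Qty and optionally destroys the owner.
; LookAt returns an empty string.
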(event EventInteractwith
  (params (PlayerRef :type BP%20Third%20Person%20Character%20Object%20Reference))
  (bind _bpc_invsystem (Variables|/Game/JACK_Content/Blueprints/BP_ThirdPersonCharacter.BP_ThirdPersonCharacter_C|GetBPC_InvSystem PlayerRef))
  (if (Variables|Default|GetisCollectable)
    ;[0 0 0 0] Check that player inventory is valid
    (Utilities|IsValid _bpc_invsystem
      (:Is%20Valid
        (bind _success (Default|AddtoInventory _bpc_invsystem (.rowname (Variables|Default|GetItemID)) (Variables|Default|GetQty)))
        (if _success
          ;[0.9569 0.1216 0 0.2235] Ensure Inventory Updates at Item Pickup
          (Default|DisplayInventory (Variables|Default|GetGrid) _bpc_invsystem)
          (Variables|Default|SetQty 0)
          (if (Variables|Default|GetDestroy)
            (Actor|DestroyActor (Components|GetOwner))))))))

(event EventBeginPlay
  ;[0 0 0 0] Enable Replication for Multiplayer
  (Networking|SetReplicates (Components|GetOwner) true)
  ;[0.9569 0.1216 0 0.2235] Delay: Ensure Grid is Made before setting variable
  (Utilities|FlowControl|DelayUntilNextTick)
  (if (Variables|Default|GetisCollectable)
    ;[0.9569 0.1216 0 0.2235] Get reference to Inventory Grid
    (bind _foundwidgets (Widget|GetAllWidgetsOfClass "/Game/JACK_Content/Blueprints/Widget/WB_InventoryGrid.WB_InventoryGrid_C" false))
    (Variables|Default|SetGrid (Utilities|Array|Get(acopy) _foundwidgets))))

(fn Lookat
  (return ""))