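; BP_LightNeeded is an actor that shows a WB_LightNeeded indicator while the player overlaps it.
; On BeginPlay it creates the widget from its Icon and Value variables, assigns it to its Widget component, caches the BP_ThirdPersonCharacter player, then hides the component.
; Begin and end overlap events toggle the component's visibility, responding only to that cached player.
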(event EventBeginPlay
  ;[0.9569 0.1216 0 0.2235] Make Widget in Actor
  (bind _returnvalue (UserInterface|CreateWidget "/Game/JACK_Content/Blueprints/Widget/WB_LightNeeded.WB_LightNeeded_C" 0 (Variables|Default|GetIcon) (Variables|Default|GetValue)))
  (UserInterface|SetWidget (Variables|Default|GetWidget) _returnvalue)
  (bind _asbp_third_person_character (Utilities|Casting|CastToBP_ThirdPersonCharacter (Game|GetPlayerCharacter 0)))
  (Variables|Default|SetPlayerRef _asbp_third_person_character)
  (Rendering|SetVisibility (Variables|Default|GetWidget) false false))

(event Collision|EventActorBeginOverlap
  (params (OtherActor :type Actor%20Object%20Reference))
  (if (== OtherActor (Variables|Default|GetPlayerRef))
    (Rendering|SetVisibility (Variables|Default|GetWidget) true false)))

(event EventTick
  (params (DeltaSeconds :type Float%20%28single-precision%29)))

(event Collision|EventActorEndOverlap
  (params (OtherActor :type Actor%20Object%20Reference))
  (if (== OtherActor (Variables|Default|GetPlayerRef))
    (Rendering|SetVisibility (Variables|Default|GetWidget) false false)))

(fn ConstructionScript)