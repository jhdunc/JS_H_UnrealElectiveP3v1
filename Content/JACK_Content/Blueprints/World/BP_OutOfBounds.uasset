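; BP_OutOfBounds is a world boundary actor with a Cube mesh that can be shown or hidden.
; Tick calls CheckBoundaryVis, which compares the VisibleBoundary flag with the cached LastSetVis and updates the Cube's visibility only when they differ.
; The graphs contain no overlap or out-of-bounds response logic.
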(event EventBeginPlay)

(event Collision|EventActorBeginOverlap
  (params (OtherActor :type Actor%20Object%20Reference)))

(event EventTick
  (params (DeltaSeconds :type Float%20%28single-precision%29))
  (CallFunction|CheckBoundaryVis))

(fn ConstructionScript)

(fn CheckBoundaryVis
  ;[0.9569 0.1216 0 0.2235] If boundary visibility bool changed, update mesh visibility
  (if (!= (Variables|Default|GetVisibleBoundary) (Variables|Default|GetLastSetVis))
    (Rendering|SetVisibility (Variables|Default|GetCube) (not (Variables|Default|GetLastSetVis)) false)
    (Variables|Default|SetLastSetVis (Variables|Default|GetVisibleBoundary))))