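; BP_InteractableUI is an interact prompt that other Blueprints position in the world.
; A Sphere's begin and end overlap events show and hide its Widget component, with no check on which actor overlaps.
; On BeginPlay it destroys the Reference component, which serves only as a positioning aid, and caches the player's BP_ThirdPersonCharacter in PlayerRef.
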(event OnComponentBeginOverlap(Sphere)
  (params (OverlappedComponent :type Primitive%20Component%20Object%20Reference) (OtherActor :type Actor%20Object%20Reference) (OtherComp :type Primitive%20Component%20Object%20Reference) (OtherBodyIndex :type Integer) (bFromSweep :type Boolean) (SweepResult :type Hit%20Result%20Structure%20%28by%20ref%29))
  ;[0.956 0.1221 0 0.2235] Show/Hide Interact Prompt
  (Rendering|SetVisibility (Variables|Default|GetWidget) true false))

(event OnComponentEndOverlap(Sphere)
  (params (OverlappedComponent :type Primitive%20Component%20Object%20Reference) (OtherActor :type Actor%20Object%20Reference) (OtherComp :type Primitive%20Component%20Object%20Reference) (OtherBodyIndex :type Integer))
  ;[0.956 0.1221 0 0.2235] Show/Hide Interact Prompt
  (Rendering|SetVisibility (Variables|Default|GetWidget) false false))

(event EventBeginPlay
  ;[0.956 0.1221 0 0.2235] Hide Reference (used to position in other BPs)
  (Components|DestroyComponent (Variables|Default|GetReference))
  (bind _asbp_third_person_character (Utilities|Casting|CastToBP_ThirdPersonCharacter (Game|GetPlayerCharacter 0)))
  (Variables|Default|SetPlayerRef _asbp_third_person_character))

(fn ConstructionScript)