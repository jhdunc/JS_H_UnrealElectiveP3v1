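; BP_MoveToGround snaps each component in its Meshes array onto the surface above or below it.
; MeshToSurface loops the array, line tracing down on the Visibility channel and retrying upward if that misses.
; On a hit, SetMeshLocation places the mesh slightly below the impact location; meshes with no hit stay put.
; Traces reach TraceDist from each mesh's world location and draw debug lines for a duration.
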(event Custom|MeshToSurface
  ;[0.9569 0.1216 0 0.2235] Move Spline to Hit Position
  (for _index (range 0 (Utilities|Array|LastIndex (Variables|Default|GetMeshes)))
    (bind _output_get (Variables|Default|SetIndex _index))
    ;;[1 0.5673 0.4162 0] Cast Down from Mesh Component
    (bind (_outhit _returnvalue) (CallFunction|LineTrace _output_get -1.0))
    ;;[1 0.5673 0.4162 0] If Hit, Move Mesh Down
    (if _returnvalue
      (CallFunction|SetMeshLocation (.Location (Collision|BreakHitResult _outhit)))
      (else
        ;;[1 0.5673 0.4162 0] If Fail, Try Up
        (bind (_outhit_2 _returnvalue_2) (CallFunction|LineTrace (Variables|Default|GetIndex) 1.0))
        (if _returnvalue_2
          (CallFunction|SetMeshLocation (.Location (Collision|BreakHitResult _outhit_2))))))))

(fn LineTrace
  (params (InputPin :type Integer) (Trace%20Direction :type Float%20%28double-precision%29))
  (bind _meshes (Variables|Default|GetMeshes))
  (bind _output (Utilities|Array|Get(acopy) _meshes InputPin))
  (bind _returnvalue (Transformation|GetWorldLocation _output))
  (bind (_outhit _returnvalue_2) (Collision|LineTraceByChannel _returnvalue (+ _returnvalue (* (Math|Vector|MakeVector 0.0 0.0 Trace%20Direction) (Variables|Default|GetTraceDist))) "TraceTypeQuery1" false 0 "ForDuration"))
  (return _outhit _returnvalue_2))

(fn SetMeshLocation
  (params (HitLocation :type Vector))
  (Transformation|SetWorldLocation (Utilities|Array|Get(acopy) (Variables|Default|GetMeshes) (Variables|Default|GetIndex)) (+ HitLocation "0.000000,0.000000,-10.000000") false false))