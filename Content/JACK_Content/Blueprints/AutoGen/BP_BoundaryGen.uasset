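; Spline-based boundary generator that spawns a row of BP_OutOfBounds actors along its path at play start.
; BeginPlay places one every ActorWidth along the spline and stores each, passing on VisibleBoundary, which BoundaryVis later toggles across all of them.
; With MoveToGround enabled, the construction script line-traces at each spline point using local-space coordinates, setting actor height from the first hit and moving other points to their hits.
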(event Custom|BoundaryVis
  ;[0.9569 0.1216 0 0.2235] Comment
  (Variables|Default|SetVisibleBoundary (not (Variables|Default|GetVisibleBoundary)))
  (for _array_element (Variables|Default|GetNewVar)
    (Variables|/Game/JACK_Content/Blueprints/World/BP_OutOfBounds.BP_OutOfBounds_C|SetVisibleBoundary _array_element (Variables|Default|GetVisibleBoundary))))

(event EventBeginPlay
  ;[0.9569 0.1216 0 0.2235] Spawn actor along Spline
  (for _index (range 0 (Math|Float|Truncate (/ (Spline|GetSplineLength (Variables|Default|GetSpline)) (Variables|Default|GetActorWidth))))
    (bind _returnvalue (Game|SpawnActorfromClass "/Game/JACK_Content/Blueprints/World/BP_OutOfBounds.BP_OutOfBounds_C" (Math|Transform|MakeTransform (.location (Spline|GetTransformatDistanceAlongSpline (Variables|Default|GetSpline) (* _index (Variables|Default|GetActorWidth)) "World" false)) (.rotation (Spline|GetTransformatDistanceAlongSpline (Variables|Default|GetSpline) (* _index (Variables|Default|GetActorWidth)) "World" false)) (.scale (Spline|GetTransformatDistanceAlongSpline (Variables|Default|GetSpline) (* _index (Variables|Default|GetActorWidth)) "World" false))) "Undefined" "MultiplyWithRoot" 0 true 0))
    (Utilities|Array|Add (Variables|Default|GetNewVar) _returnvalue)
    (Variables|/Game/JACK_Content/Blueprints/World/BP_OutOfBounds.BP_OutOfBounds_C|SetVisibleBoundary _returnvalue (Variables|Default|GetVisibleBoundary))))

(event EventTick
  (params (DeltaSeconds :type Float%20%28single-precision%29)))

(fn ConstructionScript
  ;[0 0 0 0] Comment
  (Variables|Default|SetRefresh false)
  (if (Variables|Default|GetMoveToGround)
    (CallFunction|MovePointstoGround)))

(fn MovePointstoGround
  (bind _self self)
  (bind _returnvalue (Transformation|GetActorLocation _self))
  (bind (_x _y) (Math|Vector|BreakVector _returnvalue))
  ;[0 0 0 0] The Move to Ground function I had wasn't working for non-Mesh actors, found one that did.
  (for _index (range 0 (- (Spline|GetNumberOfSplinePoints (Variables|Default|GetSpline)) 1))
    (LocalVariables|SetSplinePointIndex _index)
    (bind (_outhit _returnvalue_2) (Collision|LineTraceByChannel (+ (Spline|GetLocationatSplinePoint (Variables|Default|GetSpline) (LocalVariables|GetSplinePointIndex) "Local") "0.000000,0.000000,100000.000000") (- (Spline|GetLocationatSplinePoint (Variables|Default|GetSpline) (LocalVariables|GetSplinePointIndex) "Local") "0.000000,0.000000,20000.000000") "TraceTypeQuery1" false 0 "ForDuration"))
    (if _returnvalue_2
      (LocalVariables|SetTargetLocation (.Location (Collision|BreakHitResult _outhit)))
      (if (== (LocalVariables|GetSplinePointIndex) 0)
        (Transformation|SetActorLocation self (Math|Vector|MakeVector _x _y (.Z (Math|Vector|BreakVector (LocalVariables|GetTargetLocation)))) false false)
        (else
          (Spline|SetLocationatSplinePoint (Variables|Default|GetSpline) (LocalVariables|GetSplinePointIndex) (LocalVariables|GetTargetLocation) "World" true)))))
  (return))