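; BP_BridgeGen is a spline-based Blueprint, named as a bridge generator, that provides a MoveToSurface event to snap its spline onto the surface below.
; The event line-traces straight down from each spline point on the Visibility channel, with timed debug drawing, and moves points that hit to slightly below the impact location.
; BeginPlay and the construction script are empty, and no mesh generation appears here.
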(event Custom|MoveToSurface
  (bind _spline (Variables|Default|GetSpline))
  ;[0.9569 0.1216 0 0.2235] Move Spline to Hit Position
  (for _index (range 0 (Spline|GetNumberOfSplinePoints _spline))
    (bind _output_get (Variables|Default|SetPointIndex _index))
    ;;[0 0 0 0] Cast Down from Spline Point
    (bind (_outhit _returnvalue) (Collision|LineTraceByChannel (Spline|GetLocationatSplinePoint _spline _output_get "World") (+ (Spline|GetLocationatSplinePoint _spline _output_get "World") (* "0.000000,0.000000,-1.000000" (Variables|Default|GetTraceDist))) "TraceTypeQuery1" false 0 "ForDuration"))
    ;;[0 0 0 0] If Line Trace Hits, Move Point to Hit Location
    (if _returnvalue
      (Spline|SetLocationatSplinePoint (Variables|Default|GetSpline) (Variables|Default|GetPointIndex) (+ (.Location (Collision|BreakHitResult _outhit)) "0.000000,0.000000,-3.000000") "World" true))))

(event EventBeginPlay)

(fn ConstructionScript)