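; BP_Door is a colour-locked door from a key/door class exercise that opens by destroying itself.
; On BeginPlay it looks up its Colour enum's name in ColourTable and tints the Sphere through a dynamic material instance.
; On overlap, AttemptKey checks the BP_ThirdPersonCharacter's Keys map, and if a matching key is held, decrements that count and destroys the door.
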(event EventBeginPlay
  ;[0 0.2604 0.7135 0.152] Class Exercise: Key/Door
  ;;[0.6545 0.8168 1 0] Get color table entry from Colour name
  (Variables|Default|SetKeyColor (Utilities|Struct|MakeDataTableRowHandle "/Game/JACK_Content/CLASS/ColourTable.ColourTable" (Utilities|String|StringToName (Utilities|String|EnumtoString (Variables|Default|GetColour)))))
  ;;[0.6545 0.8168 1 0] Set material color to colour value from table ("door" type)
  (bind _returnvalue (Rendering|Material|CreateDynamicMaterialInstance (Variables|Default|GetSphere) 0 0 "None" :!class /Script/Engine.PrimitiveComponent))
  (Variables|Default|SetMaterialInstance _returnvalue)
  (bind _returnvalue_2 (Utilities|GetDataTableRow "/Game/JACK_Content/CLASS/ColourTable.ColourTable" (.rowname (Variables|Default|GetKeyColor)))
    (:then
      (Rendering|Material|SetVectorParameterValue (Variables|Default|GetMaterialInstance) "Color" (.colouroutput _returnvalue_2) :!class /Script/Engine.MaterialInstanceDynamic))))

(event Collision|EventActorBeginOverlap
  (params (OtherActor :type Actor%20Object%20Reference))
  ;[0 0.2604 0.7135 0.152] Class Exercise: Key/Door
  (CallFunction|AttemptKey OtherActor))

(fn ConstructionScript)

(fn AttemptKey
  (params (Object :type Object%20Object%20Reference))
  ;[0 0.2604 0.7135 0.152] Class Exercise: Key/Door
  ;;[0.6545 0.8168 1 0] Check Keyring against door colour
  (bind _asbp_third_person_character (Utilities|Casting|CastToBP_ThirdPersonCharacter Object))
  ;;[0.6545 0.8168 1 0] If key found, remove key from keyring and destroy actor
  (if (and (> (.Value (Utilities|Map|Find (Variables|/Game/JACK_Content/Blueprints/BP_ThirdPersonCharacter.BP_ThirdPersonCharacter_C|GetKeys _asbp_third_person_character) (Variables|Default|GetColour))) 0) (.ReturnValue (Utilities|Map|Find (Variables|/Game/JACK_Content/Blueprints/BP_ThirdPersonCharacter.BP_ThirdPersonCharacter_C|GetKeys _asbp_third_person_character) (Variables|Default|GetColour))))
    (Utilities|Map|Add (Variables|/Game/JACK_Content/Blueprints/BP_ThirdPersonCharacter.BP_ThirdPersonCharacter_C|GetKeys _asbp_third_person_character) (Variables|Default|GetColour) (- (.Value (Utilities|Map|Find (Variables|/Game/JACK_Content/Blueprints/BP_ThirdPersonCharacter.BP_ThirdPersonCharacter_C|GetKeys _asbp_third_person_character) (Variables|Default|GetColour))) 1))
    (Actor|DestroyActor)))